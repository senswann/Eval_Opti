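; Base AI enemy Blueprint that senses the player, attacks and takes damage.
; PawnSensing writes the player to the Blackboard as target, and the attack collision damages any BP_Player it overlaps.
; TakeDmg ignores hits while IsTakingDmg is set, otherwise cancelling the attack and disabling its collision.
; Helpers flag attacks, toggle a lock marker mesh and return a world location from MamberList by wrapped index.
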(event OnComponentBeginOverlap(AttackCollision)
  (params (OverlappedComponent :type Primitive%20Component%20Object%20Reference) (OtherActor :type Actor%20Object%20Reference) (OtherComp :type Primitive%20Component%20Object%20Reference) (OtherBodyIndex :type Integer) (bFromSweep :type Boolean) (SweepResult :type Hit%20Result%20Structure%20%28by%20ref%29))
  ;[1 1 1] Attack collision
  (bind _asbp_player (Utilities|Casting|CastToBP_Player OtherActor))
  (Default|TakeDmg _asbp_player (Variables|Default|GetDmg)))

(event OnSeePawn(PawnSensing)
  (params (Pawn :type Pawn%20Object%20Reference))
  ;[1 1 1] SeePlayer
  (if (== Pawn (Game|Player|GetPlayerPawn 0))
    (AI|Components|Blackboard|SetValueasObject (AI|GetBlackboard 0) (Utilities|Name|MakeLiteralName "TargetActor") (Game|Player|GetPlayerPawn 0))
    (AI|Components|Blackboard|SetValueasBool (AI|GetBlackboard 0) (Utilities|Name|MakeLiteralName "SeeingPlayer") true)))

(event EventBeginPlay)

(event Collision|EventActorBeginOverlap
  (params (OtherActor :type Actor%20Object%20Reference)))

(event EventTick
  (params (DeltaSeconds :type Float%20%28single-precision%29)))

(fn ConstructionScript)

(fn TakeDmg
  (params (Health :type Integer))
  ;[1 1 1] TakeDmg
  (if (not (Variables|Check|GetisTakingDmg?))
    (Variables|Default|SetHealth (- (Variables|Default|GetHealth) Health))
    (Variables|Check|SetisTakingDmg? true)
    (Variables|Check|SetIsAttacking? false)
    (Collision|SetCollisionEnabled (Variables|Default|GetAttackCollision) "NoCollision")))

(fn GetMamber
  (bind _mamberlist (Variables|Default|GetMamberList))
  ;[1 1 1] get mamber
  (return (Transformation|GetWorldLocation (Utilities|Array|Get(acopy) _mamberlist (Math|Integer|%(Integer) (Variables|Default|GetMamberIndex) (Utilities|Array|Length _mamberlist))))))

(fn SetLock
  ;[1 1 1] SetLock
  (Rendering|SetVisibility (Variables|Default|GetLockMesh) true false))

(fn RemoveLock
  ;[1 1 1] RemoveLock
  (Rendering|SetVisibility (Variables|Default|GetLockMesh) false false))

(fn Attack
  ;[1 1 1] Attack
  (Variables|Check|SetIsAttacking? true))