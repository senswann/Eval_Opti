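; BP_IA_BAse_High is a child AI Blueprint that registers the body parts of a character.
; Its construction script runs the parent script, then adds the center, both legs, both arms and head to MamberList.
; The event graph holds only disabled placeholder events, so the file adds no runtime logic of its own.
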(event EventBeginPlay
  (|CallParentFunction) ; This node is disabled and will not be called.\nDrag off pins to build functionality.
)

(event Collision|EventActorBeginOverlap
  (params (OtherActor :type Actor%20Object%20Reference))
  (|CallParentFunction OtherActor) ; This node is disabled and will not be called.\nDrag off pins to build functionality.
)

(event EventTick
  (params (DeltaSeconds :type Float%20%28single-precision%29))
  (|CallParentFunction DeltaSeconds) ; This node is disabled and will not be called.\nDrag off pins to build functionality.
)

(fn ConstructionScript
  (bind _mamberlist (Variables|Default|GetMamberList))
  ;[1 1 1] AddMambrer
  (|CallParentFunction)
  (Utilities|Array|Add _mamberlist (Variables|Default|GetCenter))
  (Utilities|Array|Add _mamberlist (Variables|Default|GetLeftLeg))
  (Utilities|Array|Add _mamberlist (Variables|Default|GetRigthLeg))
  (Utilities|Array|Add _mamberlist (Variables|Default|GetLeftArm))
  (Utilities|Array|Add _mamberlist (Variables|Default|GetRigthArm))
  (Utilities|Array|Add _mamberlist (Variables|Default|GetHead)))