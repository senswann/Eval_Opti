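; BP_IA_BAse_Middle is an AI base Blueprint, apparently for mid-tier enemies, that supplies body points for a lock-on marker.
; Its construction script adds Center and Head to the inherited member list.
; SetLock extends the parent version by teleporting LockMesh to the current member and turning it toward the player pawn, with 90-degree roll and yaw offsets.
; Its event graph holds only disabled default events.
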(event EventBeginPlay
  (|CallParentFunction) ; This node is disabled and will not be called.\nDrag off pins to build functionality.
)

(event Collision|EventActorBeginOverlap
  (params (OtherActor :type Actor%20Object%20Reference))
  (|CallParentFunction OtherActor) ; This node is disabled and will not be called.\nDrag off pins to build functionality.
)

(event EventTick
  (params (DeltaSeconds :type Float%20%28single-precision%29))
  (|CallParentFunction DeltaSeconds) ; This node is disabled and will not be called.\nDrag off pins to build functionality.
)

(fn ConstructionScript
  (bind _mamberlist (Variables|Default|GetMamberList))
  ;[1 1 1] addMamber
  (|CallParentFunction)
  (Utilities|Array|Add _mamberlist (Variables|Default|GetCenter))
  (Utilities|Array|Add _mamberlist (Variables|Default|GetHead)))

(fn SetLock
  (bind _returnvalue (Game|Player|GetPlayerPawn 0))
  (bind _location (CallFunction|GetMamber))
  (bind _lockmesh (Variables|Default|GetLockMesh))
  (bind _returnvalue_2 (Transformation|GetActorLocation _returnvalue))
  (bind _returnvalue_3 (Transformation|GetWorldLocation _lockmesh))
  (bind _returnvalue_4 (Math|Rotator|FindLookatRotation _returnvalue_3 _returnvalue_2))
  ;[1 1 1] Lock visibility
  (|CallParentFunction)
  (Transformation|SetWorldLocation _lockmesh (Math|Vector|MakeVector (.x _location) (.y _location) (.z _location)) false true)
  (Transformation|SetWorldRotation _lockmesh (Math|Rotator|MakeRotator (+ (.roll _returnvalue_4) 9e+01) (.pitch _returnvalue_4) (+ (.yaw _returnvalue_4) 9e+01)) false false))